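; Overview demo actor that animates a round mesh border and a round decal border to showcase runtime border updates and area checks.
; BeginPlay finds both borders and the helper actors by tag.
; Each Tick uses a sine of accumulated time to resize both borders' X size and slide them in opposite directions along Y.
; Every helper is then set active only while it lies inside either border's area.
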(event EventBeginPlay
  (bind _outactors (Actor|GetAllActorsOfClasswithTag "/Game/Resources/Art/MapBorderCollection/Blueprints/BP_Mesh_Border.BP_Mesh_Border_C" "RoundMeshBorder"))
  (Variables|Default|SetMeshBorder (Utilities|Array|Get(acopy) _outactors))
  (bind _outactors_2 (Actor|GetAllActorsOfClasswithTag "/Game/Resources/Art/MapBorderCollection/Blueprints/BP_Decal_Border.BP_Decal_Border_C" "RoundDecalBorder"))
  (Variables|Default|SetDecalBorder (Utilities|Array|Get(acopy) _outactors_2))
  (bind _outactors_3 (Actor|GetAllActorsOfClasswithTag "/Game/Resources/Art/MapBorderCollection/Overview/Blueprints/Helper/BP_Helper.BP_Helper_C" "RoundsHelper"))
  (Variables|Default|SetHelpers _outactors_3))

(event EventTick
  (params (DeltaSeconds :type Float%20%28single-precision%29))
  (if (and (Utilities|IsValid (Variables|Default|GetMeshBorder)) (Utilities|IsValid (Variables|Default|GetDecalBorder)))
    (Variables|Default|SetDeltaTIme DeltaSeconds)
    (Variables|Default|SetTime (+ (Variables|Default|GetDeltaTIme) (Variables|Default|GetTime)))
    (Utilities|FlowControl|Sequence
      (:then_0
        (Variables|/Game/Resources/Art/MapBorderCollection/Blueprints/BP_Mesh_Border.BP_Mesh_Border_C|SetBorderSIze (Variables|Default|GetMeshBorder) (Math|Vector2D|MakeVector2D (+ (+ (* (Math|Trig|Sin(Radians) (Variables|Default|GetTime)) 1e+03) 6e+02) (.Y (Math|Vector2D|BreakVector2D (Variables|/Game/Resources/Art/MapBorderCollection/Blueprints/BP_Mesh_Border.BP_Mesh_Border_C|GetBorderSIze (Variables|Default|GetMeshBorder))))) (.Y (Math|Vector2D|BreakVector2D (Variables|/Game/Resources/Art/MapBorderCollection/Blueprints/BP_Mesh_Border.BP_Mesh_Border_C|GetBorderSIze (Variables|Default|GetMeshBorder))))))
        (Variables|/Game/Resources/Art/MapBorderCollection/Blueprints/BP_Decal_Border.BP_Decal_Border_C|SetBorderSIze (Variables|Default|GetDecalBorder) (Math|Vector2D|MakeVector2D (+ (+ (* (Math|Trig|Sin(Radians) (Variables|Default|GetTime)) 1e+03) 6e+02) (.Y (Math|Vector2D|BreakVector2D (Variables|/Game/Resources/Art/MapBorderCollection/Blueprints/BP_Mesh_Border.BP_Mesh_Border_C|GetBorderSIze (Variables|Default|GetMeshBorder))))) (.Y (Math|Vector2D|BreakVector2D (Variables|/Game/Resources/Art/MapBorderCollection/Blueprints/BP_Mesh_Border.BP_Mesh_Border_C|GetBorderSIze (Variables|Default|GetMeshBorder))))))
        (Default|UpdateBorderinRuntime (Variables|Default|GetMeshBorder) false)
        (Default|UpdateBorderinRuntime (Variables|Default|GetDecalBorder))
        (Transformation|AddActorWorldOffset (Variables|Default|GetMeshBorder) (Math|Vector|MakeVector 0.0 (* (Math|Trig|Sin(Radians) (Variables|Default|GetTime)) 24.0) 0.0))
        (Transformation|AddActorWorldOffset (Variables|Default|GetDecalBorder) (Math|Vector|MakeVector 0.0 (* (* (Math|Trig|Sin(Radians) (Variables|Default|GetTime)) 24.0) -1.0) 0.0)))
      (:then_1
        (for _array_element (Variables|Default|GetHelpers)
          (bind _success (Default|CheckifPointLiesInsideArea (Variables|Default|GetMeshBorder) (Math|Conversions|ToVector2D(Vector) (Transformation|GetActorLocation _array_element))))
          (if _success
            (Default|SetNewActiveState _array_element true)
            (else
              (bind _success_2 (Default|CheckifPointLiesInsideArea (Variables|Default|GetDecalBorder) (Math|Conversions|ToVector2D(Vector) (Transformation|GetActorLocation _array_element))))
              (Default|SetNewActiveState _array_element _success_2))))))))

(fn ConstructionScript)