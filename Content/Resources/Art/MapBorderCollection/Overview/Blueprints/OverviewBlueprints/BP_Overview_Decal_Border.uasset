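; Overview demo actor that animates a tagged BP_Decal_Border at runtime to show off its properties.
; Each Tick pulses border width with a sine, eases color, corner roundness and line thickness toward targets, refreshes the border and rotates it.
; Delay and FlipFlop pairs on Tick periodically toggle rounded corners, swap colors and switch targets.
; Tagged BP_Helper actors get their active state every frame from whether they lie inside the border.
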(event EventBeginPlay
  (bind _outactors (Actor|GetAllActorsOfClasswithTag "/Game/Resources/Art/MapBorderCollection/Blueprints/BP_Decal_Border.BP_Decal_Border_C" "DecalBorder"))
  (Variables|Default|SetDecalBorder (Utilities|Array|Get(acopy) _outactors))
  (bind _outactors_2 (Actor|GetAllActorsOfClasswithTag "/Game/Resources/Art/MapBorderCollection/Overview/Blueprints/Helper/BP_Helper.BP_Helper_C" "DecalHelper"))
  (Variables|Default|SetHelpers _outactors_2))

(event EventTick
  (params (DeltaSeconds :type Float%20%28single-precision%29))
  (bind _decalborder (Variables|Default|GetDecalBorder))
  (Utilities|IsValid (Variables|Default|GetDecalBorder)
    (:Is%20Valid
      (Variables|Default|SetDeltaTIme DeltaSeconds)
      (Variables|Default|SetTime (+ (Variables|Default|GetDeltaTIme) (Variables|Default|GetTime)))
      (Variables|/Game/Resources/Art/MapBorderCollection/Blueprints/BP_Decal_Border.BP_Decal_Border_C|SetBorderSIze (Variables|Default|GetDecalBorder) (Math|Vector2D|MakeVector2D (+ (- (* (Math|Trig|Sin(Radians) (Variables|Default|GetTime)) 1e+03) 3e+02) (.Y (Math|Vector2D|BreakVector2D (Variables|/Game/Resources/Art/MapBorderCollection/Blueprints/BP_Decal_Border.BP_Decal_Border_C|GetBorderSIze (Variables|Default|GetDecalBorder))))) (.Y (Math|Vector2D|BreakVector2D (Variables|/Game/Resources/Art/MapBorderCollection/Blueprints/BP_Decal_Border.BP_Decal_Border_C|GetBorderSIze (Variables|Default|GetDecalBorder))))))
      (Variables|/Game/Resources/Art/MapBorderCollection/Blueprints/BP_Decal_Border.BP_Decal_Border_C|SetBorderColor (Variables|Default|GetDecalBorder) (Class|KismetMathLibrary|CInterpto (Variables|/Game/Resources/Art/MapBorderCollection/Blueprints/BP_Decal_Border.BP_Decal_Border_C|GetBorderColor (Variables|Default|GetDecalBorder)) (Variables|Default|GetSecondColor) (Variables|Default|GetDeltaTIme) 1.0))
      (Variables|/Game/Resources/Art/MapBorderCollection/Blueprints/BP_Decal_Border.BP_Decal_Border_C|SetCornerRoundness (Variables|Default|GetDecalBorder) (Math|Interpolation|FInterpTo (Variables|/Game/Resources/Art/MapBorderCollection/Blueprints/BP_Decal_Border.BP_Decal_Border_C|GetCornerRoundness (Variables|Default|GetDecalBorder)) (Variables|Default|GetCornerRoundnessTarget) (Variables|Default|GetDeltaTIme) 1.0))
      (Variables|/Game/Resources/Art/MapBorderCollection/Blueprints/BP_Decal_Border.BP_Decal_Border_C|SetLineThickness (Variables|Default|GetDecalBorder) (Math|Interpolation|FInterpTo (Variables|/Game/Resources/Art/MapBorderCollection/Blueprints/BP_Decal_Border.BP_Decal_Border_C|GetLineThickness (Variables|Default|GetDecalBorder)) (Variables|Default|GetLineThichnessTarget) (Variables|Default|GetDeltaTIme) 1.0))
      (Default|UpdateBorderinRuntime (Variables|Default|GetDecalBorder))
      (Transformation|AddActorLocalRotation (Variables|Default|GetDecalBorder) "0,1.000000, 0" false false)
      (Utilities|FlowControl|Sequence
        (:then_0
          (Utilities|FlowControl|Delay 2.0)
          (Utilities|FlowControl|FlipFlop
            (:A
              (Variables|/Game/Resources/Art/MapBorderCollection/Blueprints/BP_Decal_Border.BP_Decal_Border_C|SetRoundedCorners _decalborder false)
              (Variables|Default|SetSwapColor (Variables|Default|GetSecondColor))
              (Variables|Default|SetSecondColor (Variables|Default|GetFirstColor))
              (Variables|Default|SetFirstColor (Variables|Default|GetSwapColor)))
            (:B
              (Variables|/Game/Resources/Art/MapBorderCollection/Blueprints/BP_Decal_Border.BP_Decal_Border_C|SetRoundedCorners _decalborder true)
              (Variables|Default|SetSwapColor (Variables|Default|GetFirstColor))
              (Variables|Default|SetFirstColor (Variables|Default|GetSecondColor))
              (Variables|Default|SetSecondColor (Variables|Default|GetSwapColor)))))
        (:then_1
          (Utilities|FlowControl|Delay 1.3)
          (Utilities|FlowControl|FlipFlop
            (:A
              (Variables|Default|SetCornerRoundnessTarget 2e+03)
              (Variables|Default|SetLineThichnessTarget 0.3))
            (:B
              (Variables|Default|SetCornerRoundnessTarget 3e+02)
              (Variables|Default|SetLineThichnessTarget 5.0))))
        (:then_2
          (for _array_element (Variables|Default|GetHelpers)
            (bind _success (Default|CheckifPointLiesInsideArea (Variables|Default|GetDecalBorder) (Math|Conversions|ToVector2D(Vector) (Transformation|GetActorLocation _array_element))))
            (Default|SetNewActiveState _array_element _success)))))))

(fn ConstructionScript)